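; AI controller that drives a BP_Hover_Car around the spline of its assigned AI track.
; On race start it spawns an invisible target, which advances along the spline while the car is within range and wraps at the end.
; Each tick it applies full forward input and steering from a turn-angle calculation.
; If speed stays low after a short delay, it frees the car with an upward impulse and brief pitch input.
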(event Custom|Start_Race
  (Utilities|FlowControl|DoOnce false
    (:Completed
      ;[0 1 0.2449] Spawn Target Actor
      (bind _returnvalue (Game|SpawnActorfromClass "/Script/Engine.StaticMeshActor" (Math|Transform|MakeTransform "0, 0, 0" "0, 0, 0" "10.000000,10.000000,1000.000000") "Undefined" 0 0))
      (Rendering|SetVisibility (Variables|/Script/Engine.StaticMeshActor|GetStaticMeshComponent _returnvalue) false false)
      (Transformation|SetMobility _returnvalue "Movable")
      (Collision|SetCollisionEnabled (Variables|/Script/Engine.StaticMeshActor|GetStaticMeshComponent _returnvalue) "NoCollision")
      (Variables|Default|SetTargetMesh _returnvalue)
      (Components|StaticMesh|SetStaticMesh (Variables|/Script/Engine.StaticMeshActor|GetStaticMeshComponent _returnvalue) "/Game/HoverCarSystem/Vehicles/Effects/JetEngine/Meshes/SM_exhaust.SM_exhaust")
      (bind _asbp_hover_car (Utilities|Casting|CastToBP_Hover_Car (Pawn|GetControlledPawn)))
      (bind _output_get (Variables|Default|SetBP_Hover_Car _asbp_hover_car))
      (Variables|Default|SetAI_Track (Variables|/Game/HoverCarSystem/Blueprints/BP_Hover_Car.BP_Hover_Car_C|GetAI_Track _output_get)))))

(event EventTick
  (params (DeltaSeconds :type Float%20%28single-precision%29))
  (bind _bp_hover_car (Variables|Default|GetBP_Hover_Car))
  (bind _bp_hover_car_2 (Variables|Default|GetBP_Hover_Car))
  (bind _bp_hover_car_3 (Variables|Default|GetBP_Hover_Car))
  (bind _ai_track (Variables|Default|GetAI_Track))
  (bind _spline (Variables|/Game/HoverCarSystem/Blueprints/AI_Controller/BP_AI_Track.BP_AI_Track_C|GetSpline _ai_track))
  ;[0 1 0.2449] Calculate Movement
  (|CalculateDistancetoTarget)
  (Utilities|IsValid _ai_track
    (:Is%20Valid
      (if (< (Variables|Default|GetAI_Target_Distance) 3e+03)
        (bind _output_get (Variables|Default|SetDistance (+ (Variables|Default|GetDistance) (* (Variables|Default|GetAI_Target_Speed) (Utilities|Time|GetWorldDeltaSeconds))))))
      (if (> _output_get (Spline|GetSplineLength _spline))
        (Variables|Default|SetDistance 0.0))
      (bind _output_get_2 (Variables|Default|SetTarget (Spline|GetLocationatDistanceAlongSpline _spline (Variables|Default|GetDistance) "World")))
      (Transformation|SetActorLocation (Variables|Default|GetTargetMesh) _output_get_2 false false)
      (Utilities|IsValid _bp_hover_car_3
        (:Is%20Valid
          (Default|AIForward _bp_hover_car_3 1.0)
          (Default|AITurnRight (Variables|Default|GetBP_Hover_Car) (Utilities|CalculateTurnAngle (Variables|/Game/HoverCarSystem/Blueprints/BP_Hover_Car.BP_Hover_Car_C|GetCar_Physx_Mesh (Variables|Default|GetBP_Hover_Car))))
          ;[1 1 1] dont get stuck plz
          (if (Variables|Default|GetFrontUp)
            (Default|AIFrontUp _bp_hover_car -1.0)
            (Utilities|FlowControl|Delay 0.2)
            (Variables|Default|SetFrontUp false)
            (elif (< (Variables|/Game/HoverCarSystem/Blueprints/BP_Hover_Car.BP_Hover_Car_C|GetSpeed _bp_hover_car) 3e+02)
              (Utilities|FlowControl|DoOnce false :!label _label
                (:Completed
                  (Utilities|FlowControl|Delay 0.5)
                  (if (< (Variables|/Game/HoverCarSystem/Blueprints/BP_Hover_Car.BP_Hover_Car_C|GetSpeed _bp_hover_car_2) 3e+02)
                    (Physics|AddImpulse (Variables|/Game/HoverCarSystem/Blueprints/BP_Hover_Car.BP_Hover_Car_C|GetCar_Physx_Mesh _bp_hover_car_2) "0, 0,3500.000000" "None" true)
                    (Variables|Default|SetFrontUp true)
                    (goto _label Reset)
                    (else
                      (goto _label Reset))))))))))))

(fn ConstructionScript)